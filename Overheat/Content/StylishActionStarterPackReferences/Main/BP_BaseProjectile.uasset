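; Base projectile for BP_BaseCharacter owners, moved by CharacterMovement, that ignores its owner and switch characters and passes meter and style rewards back to the owner.
; Tick counts down a dilation-scaled lifetime, destroys the projectile with its hitboxes, and periodically clears hit characters for multi-hit.
; Impacts spawn sparks, stop movement and shorten lifetime, though piercing skips this for detected hits.
; Capsule hits on active characters undo sideways deflection using previous-frame velocity.
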(event `self.ReceiveBeginPlay`
  ;[1 1 1] Initialize
  (`parent.ReceiveBeginPlay`)
  (bind _asbp_base_character (cast `/Game/StylishActionStarterPackReferences/Main/BP_BaseCharacter` (`self.GetOwner`)))
  (bind _output_get (set `self.OwnerCharacter` _asbp_base_character))
  (`PrimitiveComponent.IgnoreActorWhenMoving` (`self.CapsuleComponent`) _output_get true)
  (for _array_element (`/Game/StylishActionStarterPackReferences/Main/BP_BaseCharacter.SwitchCharacters` _output_get)
    (`PrimitiveComponent.IgnoreActorWhenMoving` (`self.CapsuleComponent`) _array_element true)))

(event `Initialize`
  ;[1 1 1] Initialize
  (set `self.StyleIndex` (`/Game/StylishActionStarterPackReferences/Main/BP_BaseCharacter.SubStateIndex` (`self.OwnerCharacter`))))

(event `self.ReceiveTick`
  (params (DeltaSeconds :type "Float (single-precision)"))
  (bind _duration (`self.Duration`))
  ;[1 1 1] Update values on tick
  (`parent.ReceiveTick` DeltaSeconds)
  (`self.ResetHitsCheck`)
  (if (> _duration 0.0)
    (set `self.Duration` (`KismetMathLibrary.FClamp` (- _duration (* DeltaSeconds (`self.CustomTimeDilation`))) 0.0 _duration)))
  (if (== _duration 0.0)
    (`self.Destroy`)))

(event `ResetHitsCheck`
  ;[1 1 1] Reset hit characters for multi-hit projectiles
  (if (> (`self.MultiHitRate`) 0.0)
    (set `self.HitResetTime` (+ (`self.HitResetTime`) (* (`self.CustomTimeDilation`) (`GameplayStatics.GetWorldDeltaSeconds`))))
    (if (>= (`self.HitResetTime`) (`self.MultiHitRate`))
      (`KismetArrayLibrary.Array_Clear` (`self.HitCharacters`))
      (set `self.HitResetTime` 0.0))))

(event `CollisionEvent`
  (params (Hit :type "HitResult Structure"))
  ;[1 1 1] Called upon collision; destroys on impact by default
  (`GameplayStatics.SpawnEmitterAtLocation` "/Game/StylishActionStarterPackReferences/VFX/ParticleSystems/P_ProjectileImpactSpark.P_ProjectileImpactSpark" (`.ImpactPoint` (`GameplayStatics.BreakHitResult` Hit)))
  (set `MovementComponent.Velocity` (0.0 0.0 0.0) (`self.CharacterMovement`))
  (set `self.Duration` 0.05))

(event `self.AddMeter`
  (params (Meter :type "Float (single-precision)"))
  (bind _ownercharacter (`self.OwnerCharacter`))
  ;[1 1 1] Call on owner upon hit
  (if (not (`/Game/StylishActionStarterPackReferences/Main/BP_BaseCharacter.TriggerActive` _ownercharacter))
    (`self.AddMeter` _ownercharacter Meter)))

(event `self.AddStyle`
  (params (Index :type Integer) (Scale :type "Float (single-precision)"))
  ;[1 1 1] Call on owner upon hit
  (`self.AddStyle` (`self.OwnerCharacter`) (`self.StyleIndex`) Scale))

(event `self.CapsuleComponent.OnComponentHit`
  (params (HitComponent :type "PrimitiveComponent Object Reference") (OtherActor :type "Actor Object Reference") (OtherComp :type "PrimitiveComponent Object Reference") (NormalImpulse :type "Vector Structure") (Hit :type "HitResult Structure (by ref)"))
  (bind _returnvalue (`KismetMathLibrary.MakeRotFromX` (`self.PreviousFrameVelocity`)))
  ;[1 1 1] Called upon collision; destroys on impact by default
  (bind _asbp_base_character (cast `/Game/StylishActionStarterPackReferences/Main/BP_BaseCharacter` OtherActor)
    (:`then`
      (if (and (!= OtherActor (`self.GetOwner`)) (`/Game/StylishActionStarterPackReferences/Main/BP_BaseCharacter.Active` _asbp_base_character))
        (`PrimitiveComponent.SetCollisionEnabled` (`self.CapsuleComponent`) "NoCollision")
        (`self.K2_AddActorWorldOffset` (`KismetMathLibrary.GreaterGreater_VectorRotator` (* (- (`KismetMathLibrary.LessLess_VectorRotator` (`self.PreviousFrameLocation`) _returnvalue) (`KismetMathLibrary.LessLess_VectorRotator` (`self.K2_GetActorLocation`) _returnvalue)) (0.0 1.0 1.0)) _returnvalue))
        (`self.CollisionEvent` Hit :!label _label)))
    (:`CastFailed`
      (goto _label))))

(event `Destroy`
  ;[1 1 1] Destroy hitboxes then self
  (for _array_element (`self.Hitboxes`)
    (`self.K2_DestroyActor` _array_element))
  (`self.K2_DestroyActor`))

(event `self.HitDetected`
  (params (Hit :type "HitResult Structure"))
  ;[1 1 1] Called upon collision; destroys on impact by default
  (if (not (`self.Piercing`))
    (`self.CollisionEvent` Hit)))

(fn `UserConstructionScript`
  (`parent.UserConstructionScript`))