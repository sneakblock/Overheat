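; Player camera actor that registers with GM_CombatGameMode, becomes the view target and follows the player in free and lock-on modes.
; Each tick interpolates location, rotation and spring-arm length.
; Lock-on blends position between player and target by camera-space depth, holds yaw within a distance-scaled arc around their bearing, and zooms out as the player drifts off-center.
; Unlocked, it follows the player with clamped pitch and default arm length.
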(event `self.ReceiveBeginPlay`
  ;[1 1 1] Initialize
  (bind _asgm_combat_game_mode (cast `/Game/StylishActionStarterPackReferences/Main/GM_CombatGameMode` (`GameplayStatics.GetGameMode`)))
  (bind _output_get (set `self.GameModeRef` _asgm_combat_game_mode))
  (bind _output_get_2 (set `/Game/StylishActionStarterPackReferences/Main/GM_CombatGameMode.CameraRef` self _output_get))
  (`PlayerController.SetViewTargetWithBlend` (`GameplayStatics.GetPlayerController` 0) _output_get_2 0.0 "VTBlend_Linear" 0.0 false)
  (bind _asbp_base_character (cast `/Game/StylishActionStarterPackReferences/Main/BP_BaseCharacter` (`GameplayStatics.GetPlayerCharacter` 0)))
  (set `self.PlayerRef` _asbp_base_character))

(event `self.ReceiveTick`
  (params (DeltaSeconds :type "Float (single-precision)"))
  (`self.SetLocation`)
  (`self.SetRotation`)
  (`self.SetZoom`))

(event `SetLocation`
  (bind _playerref (`self.PlayerRef`))
  (bind _returnvalue (`self.K2_GetActorLocation` _playerref))
  (bind _returnvalue_2 (`SceneComponent.K2_GetComponentRotation` (`self.Camera`)))
  (bind _returnvalue_3 (`self.K2_GetActorLocation` (`/Game/StylishActionStarterPackReferences/Main/BP_BaseCharacter.LockOnTarget` _playerref)))
  ;[1 1 1] Update camera location
  (`/Engine/EditorBlueprintResources/StandardMacros.IsValid` _playerref
    (:`Is Valid`
      (if (`/Game/StylishActionStarterPackReferences/Main/BP_BaseCharacter.IsLockedOn` _playerref)
        (`self.K2_SetActorLocation` (`KismetMathLibrary.VInterpTo` (`self.K2_GetActorLocation`) (`KismetMathLibrary.VLerp` _returnvalue _returnvalue_3 (`KismetMathLibrary.MapRangeClamped` (- (.x (`KismetMathLibrary.LessLess_VectorRotator` _returnvalue _returnvalue_2)) (.x (`KismetMathLibrary.LessLess_VectorRotator` _returnvalue_3 _returnvalue_2))) -5000.0 5000.0 0.0 1.0)) (`GameplayStatics.GetWorldDeltaSeconds`) (* (`self.LockOnInterpSpeed`) 3.0)))
        (else
          (`self.K2_SetActorLocation` (`KismetMathLibrary.VInterpTo` (`self.K2_GetActorLocation`) (`self.K2_GetActorLocation` _playerref) (`GameplayStatics.GetWorldDeltaSeconds`) (* (`self.UnlockInterpSpeed`) 1.5))))))))

(event `SetRotation`
  (bind _returnvalue (`self.K2_GetActorRotation`))
  (bind _returnvalue_2 (`self.K2_GetActorRotation`))
  (bind _playerref (`self.PlayerRef`))
  (bind _lockontarget (`/Game/StylishActionStarterPackReferences/Main/BP_BaseCharacter.LockOnTarget` _playerref))
  (bind _returnvalue_3 (`KismetMathLibrary.MapRangeClamped` (`self.GetHorizontalDistanceTo` _playerref _lockontarget) 300.0 1000.0 179.0 20.0))
  (bind _returnvalue_4 (`KismetMathLibrary.MakeRotator` 0.0 0.0 (.yaw (`KismetMathLibrary.FindLookAtRotation` (`self.K2_GetActorLocation` _playerref) (`self.K2_GetActorLocation` _lockontarget)))))
  ;[1 1 1] Update camera rotation
  (if (`/Game/StylishActionStarterPackReferences/Main/BP_BaseCharacter.IsLockedOn` (`self.PlayerRef`))
    (`self.K2_SetActorRotation` (`KismetMathLibrary.RInterpTo` _returnvalue_2 (`KismetMathLibrary.MakeRotator` 0.0 -15.0 (`KismetMathLibrary.ClampAngle` (.yaw _returnvalue_2) (.yaw (`KismetMathLibrary.ComposeRotators` _returnvalue_4 (`KismetMathLibrary.MakeRotator` 0.0 0.0 (* _returnvalue_3 -1.0)))) (.yaw (`KismetMathLibrary.ComposeRotators` _returnvalue_4 (`KismetMathLibrary.MakeRotator` 0.0 0.0 _returnvalue_3))))) (`GameplayStatics.GetWorldDeltaSeconds`) (`self.LockOnInterpSpeed`)))
    (else
      (`self.K2_SetActorRotation` (`KismetMathLibrary.RInterpTo` _returnvalue (`KismetMathLibrary.MakeRotator` 0.0 (`KismetMathLibrary.FClamp` (.pitch _returnvalue) -60.0 60.0) (.yaw _returnvalue)) (`GameplayStatics.GetWorldDeltaSeconds`) 30.0)))))

(event `SetZoom`
  (bind _camera (`self.Camera`))
  ;[1 1 1] Update camera zoom
  (if (`/Game/StylishActionStarterPackReferences/Main/BP_BaseCharacter.IsLockedOn` (`self.PlayerRef`))
    (set `SpringArmComponent.TargetArmLength` (`KismetMathLibrary.FInterpTo` (`SpringArmComponent.TargetArmLength` (`self.SpringArm`)) (+ (* (- 1.0 (`KismetMathLibrary.Dot_VectorVector` (1.0 0.0 0.0) (`KismetMathLibrary.Normal` (* (`KismetMathLibrary.LessLess_VectorRotator` (`KismetMathLibrary.GetDirectionUnitVector` (`SceneComponent.K2_GetComponentLocation` _camera) (`self.K2_GetActorLocation` (`self.PlayerRef`))) (`SceneComponent.K2_GetComponentRotation` _camera)) (1.0 1.0 2.0))))) 2500.0) (`self.LockonArmLengthOffset`)) (`GameplayStatics.GetWorldDeltaSeconds`) (`self.LockOnInterpSpeed`)) (`self.SpringArm`))
    (else
      (set `SpringArmComponent.TargetArmLength` (`KismetMathLibrary.FInterpTo` (`SpringArmComponent.TargetArmLength` (`self.SpringArm`)) (`self.DefaultArmLength`) (`GameplayStatics.GetWorldDeltaSeconds`) (`self.UnlockInterpSpeed`)) (`self.SpringArm`)))))

(fn `UserConstructionScript`)