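; BP_OverdriveProjectile is a projectile Blueprint, named for an Overdrive attack, that configures multiple hitboxes to deal light, repeatable-scale hits with an upward launch.
; It overrides Initialize, calling the parent first, then loops over the inherited Hitboxes array.
; Each hitbox gets shared hit data, a sphere radius and an index-based offset forming a three-point arrowhead, then activates.
; All other behavior comes from the parent class.
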(event `/Game/StylishActionStarterPackReferences/Main/BP_BaseProjectile.Initialize`
  ;[1 1 1] Initialize
  (`parent.Initialize`)
  (for (_array_element _array_index) (`self.Hitboxes`)
    (set `/Game/StylishActionStarterPackReferences/Misc/BP_Hitbox.HitData` (make `/Game/StylishActionStarterPackReferences/Main/Structs/Struct_HitData` 0 (0.0 0.0 200.0) 2.0 1 0.001 0.02 1.0) _array_element)
    (`SphereComponent.SetSphereRadius` (`/Game/StylishActionStarterPackReferences/Misc/BP_Hitbox.Hitbox` _array_element) 75.0 true)
    (`self.K2_SetActorRelativeLocation` _array_element (select `int` _array_index :`0` (0.0 0.0 0.0) :`1` (-50.0 100.0 0.0) :`2` (-50.0 -100.0 0.0) :!type "Vector Structure") false false)
    (`/Game/StylishActionStarterPackReferences/Misc/BP_Hitbox.Activate` _array_element true)))

(fn `UserConstructionScript`
  (`parent.UserConstructionScript`))