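; Taunt enemy character that keeps a permanent lock-on to the player and plays reactive moves instead of real attacks.
; When grounded and able to attack, its melee input uses the AI controller's action index to pick a back dodge, guard-hit or taunt montage.
; It fakes directional input from the camera-relative direction to the player, reversed for the dodge and zeroed for the guard.
; A timed charge-and-release attack path remains unconnected.
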(event `self.ReceiveBeginPlay`
  ;[1 1 1] Initialize
  (`parent.ReceiveBeginPlay`)
  (bind _asbp_base_character (cast `/Game/Main/BP_BaseCharacter` (`GameplayStatics.GetPlayerCharacter` 0)))
  (set `self.LockOnTarget` _asbp_base_character)
  (set `self.IsLockedOn` true)
  (set `self.LockonButton` true))

(event `self.InputMelee`
  (params (Pressed :type Boolean) (isHeavy :type Boolean))
  (bind (_x _y) (`KismetMathLibrary.BreakVector2D` (`KismetMathLibrary.Conv_VectorToVector2D` (`KismetMathLibrary.LessLess_VectorRotator` (`KismetMathLibrary.Normal` (`KismetMathLibrary.MakeVector` (.x (`KismetMathLibrary.GetDirectionUnitVector` (`self.K2_GetActorLocation`) (`self.K2_GetActorLocation` (`self.LockOnTarget`)))) (.y (`KismetMathLibrary.GetDirectionUnitVector` (`self.K2_GetActorLocation`) (`self.K2_GetActorLocation` (`self.LockOnTarget`)))))) (`self.CameraYaw`)))))
  (bind _returnvalue (`KismetMathLibrary.MakeVector2D` _y _x))
  ;[1 1 1] Attack command
  (if (`self.CanAttack`)
    (if (not (`self.InAir`))
      ;;[1 1 1] Set input vector to simulate directional inputs
      (set `self.InputVector` (select `int` (`/Game/Ai/AIC_Enemy.AIActionIndex` (`self.AIControllerRef`)) :`0` (* _returnvalue -1.0) :`1` (0.0 0.0) :`2` _returnvalue))
      (switch `int` (`/Game/Ai/AIC_Enemy.AIActionIndex` (`self.AIControllerRef`))
        (:`Default`
          (`self.CanDo` true))
        (:`0`
          ;[1 1 1] Simulated Melee Input
          (`self.PlayAnimMontage` "/Game/Characters/FighterAnimations/Movement/Fighter_Dodge_B_Montage.Fighter_Dodge_B_Montage" 1.0 "None")
          (`self.UpdateRecentMoves` -1 :!label _label))
        (:`1`
          (`self.PlayAnimMontage` "/Game/Characters/FighterAnimations/Defense/Fighter_Guard_hit_air_Montage.Fighter_Guard_hit_air_Montage" 1.0 "None")
          (goto _label))
        (:`2`
          ;;[1 1 1] Taunt
          (`self.PlayAnimMontage` "/Game/AmriDev/TauntEnemy/Fighter_Taunt_Montage2.Fighter_Taunt_Montage2" 1.0 "None")
          (goto _label))))))

(event `CustomEvent`
  ;[1 1 1] Input attack button and hold for specified charge time
  (bind _output_get (set `self.MeleeButton` false))
  (`parent.InputMelee` _output_get false)
  (bind _output_get_2 (set `self.SpecialButton` false))
  (`parent.InputSpecial` _output_get_2))

(fn `UserConstructionScript`
  (`parent.UserConstructionScript`))