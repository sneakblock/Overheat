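; Player lock-on reticle Blueprint that tracks the currently targeted character and exposes that target's health.
; It extends the parent's attach and detach events, caching the target when it casts to BP_BaseCharacter and clearing it on detach.
; GetTargetFractionOfHealth returns the cached target's Health divided by MaxHealth when that target is valid.
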(event `self.AttachToNewTarget`
  (params (TargetCharacter :type "Character Object Reference"))
  (`parent.AttachToNewTarget` TargetCharacter)
  (bind _asbp_base_character (cast `/Game/Main/BP_BaseCharacter` TargetCharacter))
  (set `self.LockOnTarget` _asbp_base_character))

(event `self.DetachFromTarget`
  (`parent.DetachFromTarget`)
  (set `self.LockOnTarget` null) ; Set to null
)

(fn `GetTargetFractionOfHealth`
  (returns (ReturnValue :type "Float (double-precision)"))
  (bind _lockontarget (`self.LockOnTarget`))
  (`/Engine/EditorBlueprintResources/StandardMacros.IsValid` _lockontarget
    (:`Is Valid`
      (return (/ (`/Game/Main/BP_BaseCharacter.Health` _lockontarget) (`/Game/Main/BP_BaseCharacter.MaxHealth` _lockontarget))))))