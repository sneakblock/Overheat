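; Final double doors that toggle once all enemy spawners are exhausted and no enemies remain.
; On BeginPlay it gathers every BP_BaseEnemySpawner, caches the combat game mode and starts a looping timer instead of using Tick.
; Each check requires empty EnemiesToSpawn lists on all spawners and an empty game mode Enemies list, then pauses the timer and calls ToggleDoor.
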(event `self.ReceiveBeginPlay`
  (`parent.ReceiveBeginPlay`)
  (bind _outactors (`GameplayStatics.GetAllActorsOfClass` "/Game/AI/Spawners/BP_BaseEnemySpawner.BP_BaseEnemySpawner_C"))
  (set `self.EnemySpawners` _outactors)
  (bind _returnvalue (`KismetSystemLibrary.K2_SetTimerDelegate` (delegate `CheckSpawnerState`) 3.0 true))
  (set `self.SpawnerTimerHandle` _returnvalue)
  (bind _asgm_combat_game_mode (cast `/Game/Main/GM_CombatGameMode` (`GameplayStatics.GetGameMode`)))
  (set `self.GameModeRef` _asgm_combat_game_mode)
  (set `self.open` false))

(event `CheckSpawnerState`
  (set `self.ShouldOpen` true)
  (for _array_element (`self.EnemySpawners`)
    (if (> (`KismetArrayLibrary.Array_Length` (`/Game/AI/Spawners/BP_BaseEnemySpawner.EnemiesToSpawn` _array_element)) 0)
      (set `self.ShouldOpen` false)))
  (if (and (`self.ShouldOpen`) (<= (`KismetArrayLibrary.Array_Length` (`/Game/Main/GM_CombatGameMode.Enemies` (`self.GameModeRef`))) 0))
    (`KismetSystemLibrary.K2_PauseTimerHandle` (`self.SpawnerTimerHandle`))
    (`self.ToggleDoor`)))

(fn `UserConstructionScript`
  (`parent.UserConstructionScript`))