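; Default game mode that populates the level with player pawns and sets up the HUD when play begins.
; BeginPlay spawns a PlayerBlueprint at every PlayerStart through SpawnPlayer, then creates a HUD widget for the first player controller and adds it to the viewport.
; It finally destroys every PlayerBlueprint that is not player-controlled, so only possessed pawns remain.
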(event `self.ReceiveBeginPlay`
  (bind _outactors (`GameplayStatics.GetAllActorsOfClass` "/Script/Engine.PlayerStart"))
  (for _array_element _outactors
    (`self.SpawnPlayer` _array_element))
  (bind _returnvalue (`|CreateWidget` "/Game/Blueprints/PlayerHUD.PlayerHUD_C" (`GameplayStatics.GetPlayerController` 0)))
  (`UserWidget.AddToViewport` _returnvalue 0)
  (bind _outactors_2 (`GameplayStatics.GetAllActorsOfClass` "/Game/Blueprints/PlayerBlueprint.PlayerBlueprint_C"))
  (for _array_element_2 _outactors_2
    (if (not (`Pawn.IsPlayerControlled` _array_element_2))
      (`self.K2_DestroyActor` _array_element_2))))

(fn `SpawnPlayer`
  (params (playerStart :type "PlayerStart Object Reference"))
  (`|SpawnActorFromClass` "/Game/Blueprints/PlayerBlueprint.PlayerBlueprint_C" (`self.GetTransform` playerStart) "Undefined" "OverrideRootScale" null null))

(fn `UserConstructionScript`)