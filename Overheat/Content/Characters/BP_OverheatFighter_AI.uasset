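; AI-controlled Overheat Fighter that locks onto the player at BeginPlay and attacks by simulating player inputs on its parent character.
; When able to attack on the ground, InputMelee uses the controller's AIActionIndex to fake a camera-relative stick direction away from, neutral or toward the target.
; It presses Special for the neutral action and Melee otherwise, then a timer releases both buttons after a short charge hold.
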(event `self.ReceiveBeginPlay`
  ;[1 1 1] Initialize
  (`parent.ReceiveBeginPlay`)
  (bind _asbp_base_character (cast `/Game/StylishActionStarterPackReferences/Main/BP_BaseCharacter` (`GameplayStatics.GetPlayerCharacter` 0)))
  (set `self.LockOnTarget` _asbp_base_character)
  (set `self.IsLockedOn` true)
  (set `self.LockonButton` true))

(event `self.InputMelee`
  (params (Pressed :type Boolean))
  (bind _aiactionindex (`/Game/StylishActionStarterPackReferences/AI/AIC_Enemy.AIActionIndex` (`self.AIControllerRef`)))
  (bind (_x _y) (`KismetMathLibrary.BreakVector2D` (`KismetMathLibrary.Conv_VectorToVector2D` (`KismetMathLibrary.LessLess_VectorRotator` (`KismetMathLibrary.Normal` (`KismetMathLibrary.MakeVector` (.x (`KismetMathLibrary.GetDirectionUnitVector` (`self.K2_GetActorLocation`) (`self.K2_GetActorLocation` (`self.LockOnTarget`)))) (.y (`KismetMathLibrary.GetDirectionUnitVector` (`self.K2_GetActorLocation`) (`self.K2_GetActorLocation` (`self.LockOnTarget`)))))) (`self.CameraYaw`)))))
  (bind _returnvalue (`KismetMathLibrary.MakeVector2D` _y _x))
  ;[1 1 1] Attack command
  (if (`self.CanAttack`)
    (if (not (`self.InAir`))
      ;;[1 1 1] Set input vector to simulate directional inputs
      (set `self.InputVector` (select `int` _aiactionindex :`0` (* _returnvalue -1.0) :`1` (0.0 0.0) :`2` _returnvalue))
      ;;[1 1 1] Input attack button and hold for specified charge time
      (if (== _aiactionindex 1)
        (bind _output_get (set `self.SpecialButton` true))
        (`parent.InputSpecial` _output_get)
        (else
          (bind _output_get_2 (set `self.MeleeButton` true))
          (`parent.InputMelee` _output_get_2)))
      (`KismetSystemLibrary.K2_SetTimerDelegate` (delegate `ChargeTimer`) 0.5))))

(event `ChargeTimer`
  ;[1 1 1] Attack command
  ;;[1 1 1] Input attack button and hold for specified charge time
  (bind _output_get (set `self.MeleeButton` false))
  (`parent.InputMelee` _output_get)
  (bind _output_get_2 (set `self.SpecialButton` false))
  (`parent.InputSpecial` _output_get_2))

(fn `UserConstructionScript`
  (`parent.UserConstructionScript`))