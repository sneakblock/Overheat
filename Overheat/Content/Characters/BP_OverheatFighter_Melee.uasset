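; Melee fighter character Blueprint for Overheat Fighter, adding a toggleable burst trigger and a red tag-in effect on top of its parent.
; Burst input activates the trigger when the fighter is alive, off cooldown and at full meter, spending half the meter, and can switch it off early.
; Each toggle updates red VFX, sound and play rate (faster while active), clears the hit-character list and restarts the cooldown.
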(event `self.InputBurst`
  (params (Pressed :type Boolean))
  (bind _triggeractive (`self.TriggerActive`))
  (bind _returnvalue (== (`self.TriggerCooldownTimer`) 0.0))
  ;[1 1 1] Passive burst activation
  (if Pressed
    (if (and _returnvalue (>= (`self.Meter`) 100.0) (> (`self.Health`) 0.0))
      (`self.TriggerActivate` (not _triggeractive))
      (elif (and _triggeractive _returnvalue)
        (`self.TriggerActivate` false)))))

(event `self.TriggerActivate`
  (params (Active :type Boolean))
  ;[1 1 1] Passive burst activation
  (bind _output_get (set `self.TriggerActive` Active))
  (`self.PlayPassiveVFX` _output_get 0 "/Game/StylishActionStarterPackReferences/VFX/ParticleSystems/P_TriggerRed.P_TriggerRed" (struct) "pelvis")
  (`GameplayStatics.SpawnSoundAttached` (select `bool` _output_get :!type "SoundBase Object Reference") (`self.Mesh`) "None" (0.0 0.0 0.0) (struct) "KeepRelativeOffset" false (select `bool` _output_get :`false` 1.0 :`true` 1.5 :!type "Float (single-precision)") 1.0 0.0 null null)
  (set `self.CharacterPlayRate` (`KismetMathLibrary.SelectFloat` 1.2 1.0 (`self.TriggerActive`)))
  (`KismetArrayLibrary.Array_Clear` (`self.HitCharacters`))
  (set `self.TriggerCooldownTimer` (`self.TriggerCooldown`))
  (if (`self.TriggerActive`)
    (`self.AddMeter` -50.0)))

(event `self.TagIn`
  ;[1 1 1] Tag in VFX
  (bind _returnvalue (`GameplayStatics.SpawnEmitterAttached` "/Game/StylishActionStarterPackReferences/VFX/ParticleSystems/P_SwitchRed.P_SwitchRed" (`self.Mesh`) "pelvis"))
  (set `SceneComponent.bAbsoluteRotation` true _returnvalue))

(fn `UserConstructionScript`
  (`parent.UserConstructionScript`))