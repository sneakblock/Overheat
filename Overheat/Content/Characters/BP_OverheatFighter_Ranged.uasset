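; Ranged fighter character that overrides its parent's special, hit, double-jump and dodge behavior with projectile moves.
; Directional input picks montage-driven specials (Ki Slash, back-input projectiles) with air variants, buffering input when actions are unavailable and setting state indices.
; Perfect-timed hits in the counter state trigger an invincible projectile counter; double jumps spawn a projectile below.
; Dodge gives invincible dashes, limited in air, while forward input starts a teleport.
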(event `self.InputSpecial`
  (params (Pressed :type Boolean))
  (bind _charactermovement (`self.CharacterMovement`))
  (bind _charactermovement_2 (`self.CharacterMovement`))
  ;[1 1 1] Special Input
  (if Pressed
    (if (`self.CanAttack`)
      (`self.StartAnim`)
      (`self.CanDo` false)
      (`self.OrientCharacter` true)
      (if (`self.InAir`)
        ;[1 1 1] Special Air Moves
        (switch `int` (+ (select `bool` (== (`self.InputBuffer`) 4) :`false` (`self.DirectionalInput`) :`true` (`self.DirectionBuffer`)) 1)
          (:`0`
            ;;[1 1 1] Back Input: Hammer Projectile
            (`self.PlayAnimMontage` "/Game/StylishActionStarterPackReferences/Characters/FighterAnimations/Attacks/Fighter_HammerProjectile_Montage.Fighter_HammerProjectile_Montage" 1.0 "None")
            (set `self.StateIndex` 2)
            (set `self.SubStateIndex` 31)
            (set `CharacterMovementComponent.GravityScale` 2.0 _charactermovement_2)
            (set `MovementComponent.Velocity` (+ (* (`MovementComponent.Velocity` _charactermovement_2) (0.5 0.5 0.0)) (0.0 0.0 300.0)) _charactermovement_2)
            (set `self.FloatTime` 0.3))
          (:`1`
            ;;[1 1 1] Neutral Input: Ki Slash (Air)
            (`self.PlayAnimMontage` "/Game/StylishActionStarterPackReferences/Characters/FighterAnimations/Attacks/Fighter_KiSlash_air_Montage.Fighter_KiSlash_air_Montage" 1.0 "None" :!label _label)
            (set `self.StateIndex` 2)
            (set `self.SubStateIndex` 35)
            (set `CharacterMovementComponent.GravityScale` 2.0 _charactermovement)
            (set `MovementComponent.Velocity` (+ (* (`MovementComponent.Velocity` _charactermovement) (0.5 0.5 0.0)) (0.0 0.0 200.0)) _charactermovement)
            (set `self.FloatTime` 0.3))
          (:`2`
            (goto _label)))
        (`self.UpdateRecentMoves` -1)
        (else
          ;[1 1 1] Special Ground Moves
          (switch `int` (+ (select `bool` (== (`self.InputBuffer`) 4) :`false` (`self.DirectionalInput`) :`true` (`self.DirectionBuffer`)) 1)
            (:`0`
              ;;[1 1 1] Back Input: Rush Projectiles
              (`self.PlayAnimMontage` "/Game/StylishActionStarterPackReferences/Characters/FighterAnimations/Attacks/Fighter_RushProjectiles_Montage.Fighter_RushProjectiles_Montage" 1.0 "None")
              (set `self.StateIndex` 2)
              (set `self.SubStateIndex` 25))
            (:`1`
              ;;[1 1 1] Neutral Input: Ki Slash
              (`self.PlayAnimMontage` "/Game/StylishActionStarterPackReferences/Characters/FighterAnimations/Attacks/Fighter_KiSlash.Fighter_KiSlash" 1.0 "None" :!label _label_2)
              (set `self.StateIndex` 2)
              (set `self.SubStateIndex` 20))
            (:`2`
              (goto _label_2)))
          (`self.UpdateRecentMoves` -1)))
      (elif (>= (`self.InputBuffer`) 0)
        (set `self.InputBuffer` 4)
        (set `self.DirectionBuffer` (`self.DirectionalInput`))))
    (elif (`self.SpecialCharge`)
      (`self.SpecialChargeRelease`))))

(event `self.GetHit`
  (params (HitData :type "/Game/StylishActionStarterPackReferences/Main/Structs/Struct_HitData Structure") (AttackerHitbox :type "/Game/StylishActionStarterPackReferences/Misc/BP_Hitbox Object Reference") (HitResult :type "HitResult Structure"))
  (bind _charactermovement (`self.CharacterMovement`))
  ;[1 1 1] Counter Activation
  (if (and (<= (`self.GuardTime`) (`self.PerfectGuardTime`)) (== (`self.StateIndex`) 3) (== (`self.SubStateIndex`) 1))
    (`self.PlayAnimMontage` (select `bool` (`self.InAir`) :`false` "/Game/StylishActionStarterPackReferences/Characters/FighterAnimations/Defense/Fighter_Counter_Projectile_just_Montage.Fighter_Counter_Projectile_just_Montage" :`true` "/Game/StylishActionStarterPackReferences/Characters/FighterAnimations/Defense/Fighter_Counter_Projectile_air_just_Montage.Fighter_Counter_Projectile_air_just_Montage" :!type "AnimMontage Object Reference") 1.0 "Start")
    (`self.StartAnim`)
    (`self.CanDo` false)
    (`self.RestoreMovementDefaults` true)
    (`self.OrientCharacter` true)
    (set `self.StateIndex` 3)
    (set `self.SubStateIndex` 2)
    (set `self.InputBuffer` 0)
    (`self.SetInvinciblity` true)
    (if (`self.InAir`)
      (set `self.FloatTime` 0.3)
      (set `MovementComponent.Velocity` (0.0 0.0 10.0) _charactermovement)
      (set `CharacterMovementComponent.GravityScale` 0.0 _charactermovement)
      (set `CharacterMovementComponent.FallingLateralFriction` 2.0 _charactermovement))
    (else
      (`parent.GetHit` HitData AttackerHitbox (struct)))))

(event `self.DoubleJumpEffect`
  ;[1 1 1] Double jump projectile
  (bind _returnvalue (`|SpawnActorFromClass` "/Game/StylishActionStarterPackReferences/Projectiles/BP_JumpProjectile.BP_JumpProjectile_C" (`KismetMathLibrary.MakeTransform` (+ (`self.K2_GetActorLocation`) (0.0 0.0 -90.0))) "AlwaysSpawn" "OverrideRootScale" self null))
  (`self.SpawnDefaultController` _returnvalue)
  (`/Game/StylishActionStarterPackReferences/Main/BP_BaseProjectile.Initialize` _returnvalue)
  (`self.UpdateRecentMoves` 50))

(event `self.InputDodge`
  (params (Pressed :type Boolean))
  (bind _charactermovement (`self.CharacterMovement`))
  (bind _charactermovement_2 (`self.CharacterMovement`))
  (bind _returnvalue (== (`self.DirectionalInput`) -1))
  ;[1 1 1] Dodge
  (if Pressed
    (if (`self.AbleToJump`)
      (switch `int` (+ (select `bool` (== (`self.InputBuffer`) 2) :`false` (`self.DirectionalInput`) :`true` (`self.DirectionBuffer`)) 1)
        (:`0`
          (if (or (< (`self.AirDashesUsed`) (select `bool` (`self.TriggerActive`) :`false` 1 :`true` 2)) (not (`self.InAir`))) :!label _label_3
            (`self.OrientCharacter` (or (<= (`KismetMathLibrary.VSize2D` (`self.InputVector`)) (`self.WalkThreshold`)) (!= (`self.DirectionalInput`) 0)) false)
            (`self.StartAnim`)
            (`self.CanDo` false)
            (if (`self.InAir`)
              (`self.PlayAnimMontage` (select `bool` _returnvalue :`false` "/Game/StylishActionStarterPackReferences/Characters/FighterAnimations/Movement/Fighter_Dodge_air_F_Montage.Fighter_Dodge_air_F_Montage" :`true` "/Game/StylishActionStarterPackReferences/Characters/FighterAnimations/Movement/Fighter_Dodge_air_B_Montage.Fighter_Dodge_air_B_Montage" :!type "AnimMontage Object Reference"))
              (`/Engine/EditorBlueprintResources/StandardMacros.IncrementInt` (`self.AirDashesUsed`)
                (:`  `
                  (set `CharacterMovementComponent.GravityScale` 0.0 _charactermovement)
                  (set `self.FloatTime` 0.5)
                  (set `MovementComponent.Velocity` (0.0 0.0 1.0) _charactermovement)))
              (else
                (`self.PlayAnimMontage` (select `bool` _returnvalue :`false` "/Game/StylishActionStarterPackReferences/Characters/FighterAnimations/Movement/Fighter_Dodge_F_Montage.Fighter_Dodge_F_Montage" :`true` "/Game/StylishActionStarterPackReferences/Characters/FighterAnimations/Movement/Fighter_Dodge_B_Montage.Fighter_Dodge_B_Montage" :!type "AnimMontage Object Reference"))))
            (set `self.StateIndex` 1)
            (set `self.SubStateIndex` 1)
            (set `self.Invincible` true)))
        (:`1`
          (goto _label_3))
        (:`2`
          ;;[1 1 1] Teleport
          (`self.StartAnim`)
          (`self.RestoreMovementDefaults` true)
          (`self.OrientCharacter` true false)
          (set `MovementComponent.Velocity` (+ (* (`self.GetActorForwardVector`) 50.0) (0.0 0.0 100.0)) _charactermovement_2)
          (set `self.FloatTime` 0.2)
          (set `CharacterMovementComponent.GravityScale` 2.0 _charactermovement_2)
          (set `self.StateIndex` 1)
          (set `self.SubStateIndex` 10)
          (set `self.Invincible` true)
          (set `self.CombatAnimation` false)
          (`self.PlayAnimMontage` "/Game/StylishActionStarterPackReferences/Characters/FighterAnimations/Movement/Fighter_TeleportGround_Montage.Fighter_TeleportGround_Montage" 1.0 "Start")
          (set `self.InputBuffer` 0)
          (`self.CanDo` false)
          (`GameplayStatics.SpawnEmitterAtLocation` "/Game/StylishActionStarterPackReferences/VFX/ParticleSystems/P_TeleportBlue.P_TeleportBlue" (`self.K2_GetActorLocation`))))
      (elif (>= (`self.InputBuffer`) 0)
        (set `self.InputBuffer` 2)
        (set `self.DirectionBuffer` (`self.DirectionalInput`))))))

(fn `UserConstructionScript`
  (`parent.UserConstructionScript`))