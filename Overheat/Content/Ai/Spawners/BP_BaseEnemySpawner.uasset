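; Enemy spawner for combat encounters that locks an area with doors when the player's fighter enters a one-shot trigger.
; A looping timer spawns mannequin AI at random points in SpawnVolume while the controller count is below MaxEnemies, registering each with the game mode and AI manager.
; A second timer toggles the doors again and pauses itself once the game mode's enemy list empties, leaving the spawn timer running.
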(event `SpawnEnemy`
  (bind _spawnvolume (`self.SpawnVolume`))
  (bind _aimanager (`self.AiManager`))
  (bind _outactors (`GameplayStatics.GetAllActorsOfClass` "/Game/AI/AIC_Mannequin.AIC_Mannequin_C"))
  (if (< (`KismetArrayLibrary.Array_Length` _outactors) (`self.Max Enemies`))
    (bind _returnvalue (`AIBlueprintHelperLibrary.SpawnAIFromClass` "/Game/Characters/BP_MannequinFighter_AI.BP_MannequinFighter_AI_C" "/Game/AI/BT_Mannequin.BT_Mannequin" (`KismetMathLibrary.RandomPointInBoundingBox` (`SceneComponent.K2_GetComponentLocation` _spawnvolume) (`BoxComponent.GetScaledBoxExtent` _spawnvolume))))
    (bind _asgm_combat_game_mode (cast `/Game/Main/GM_CombatGameMode` (`GameplayStatics.GetGameMode`)))
    (bind _asbp_base_character (cast `/Game/Main/BP_BaseCharacter` _returnvalue))
    (`KismetArrayLibrary.Array_AddUnique` (`/Game/Main/GM_CombatGameMode.Enemies` _asgm_combat_game_mode) _asbp_base_character)
    (`KismetArrayLibrary.Array_AddUnique` (`/Game/AI/BP_AI_Manager.AI_Characters` _aimanager) _asbp_base_character)
    (set `/Game/Main/BP_BaseCharacter.AI_Manager` _aimanager _asbp_base_character)
    (bind _asaic_enemy (cast `/Game/AI/AIC_Enemy` (`AIBlueprintHelperLibrary.GetAIController` _asbp_base_character)))
    (set `/Game/AI/AIC_Enemy.ControlledCharacter` _asbp_base_character _asaic_enemy)
    (else
      (`KismetSystemLibrary.PrintString` "False"))))

(event `self.ReceiveBeginPlay`
  (bind _returnvalue (`GameplayStatics.GetActorOfClass` "/Game/AI/BP_AI_Manager.BP_AI_Manager_C"))
  (set `self.AiManager` _returnvalue)
  (bind _asgm_combat_game_mode (cast `/Game/Main/GM_CombatGameMode` (`GameplayStatics.GetGameMode`)))
  (set `self.GameModeReference` _asgm_combat_game_mode))

(event `self.Trigger.OnComponentBeginOverlap`
  (params (OverlappedComponent :type "PrimitiveComponent Object Reference") (OtherActor :type "Actor Object Reference") (OtherComp :type "PrimitiveComponent Object Reference") (OtherBodyIndex :type Integer) (bFromSweep :type Boolean) (SweepResult :type "HitResult Structure (by ref)"))
  (cast `/Game/Characters/BP_MannequinFighter` OtherActor)
  (`self.StartSpawning`)
  (`ActorComponent.K2_DestroyComponent` (`self.Trigger`))
  (bind _returnvalue (`KismetSystemLibrary.K2_SetTimerDelegate` (delegate `CheckEnemiesAlive`) 1.0 true))
  (set `self.EnemyCheckTimerHandle` _returnvalue))

(event `StartSpawning`
  ;[1 1 1] Sets the spawner to start spawning stuff
  (`KismetSystemLibrary.K2_SetTimer` null "SpawnEnemy" (/ 1.0 (`self.EnemiesPerSecond`)) true)
  (for _array_element (`self.Door References`)
    (`BaseDoor.ToggleDoor` _array_element)))

(event `CheckEnemiesAlive`
  (if (<= (`KismetArrayLibrary.Array_Length` (`/Game/Main/GM_CombatGameMode.Enemies` (`self.GameModeReference`))) 0)
    (for _array_element (`self.Door References`)
      (`BaseDoor.ToggleDoor` _array_element))
    (`KismetSystemLibrary.K2_PauseTimerHandle` (`self.EnemyCheckTimerHandle`))))

(fn `UserConstructionScript`)