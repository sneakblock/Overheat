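; Ki slash projectile, a child Blueprint that configures its inherited hitboxes and initial aim on Initialize.
; Each hitbox gets light damage, an upward launch and a sphere radius, then is offset forward, up or down by index and activated.
; When the owner is locked on to a valid target, it redirects velocity along the owner-to-target direction at unchanged speed and adjusts only its pitch to match.
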(event `self.Initialize`
  (bind _ownercharacter (`self.OwnerCharacter`))
  (bind _ownercharacter_2 (`self.OwnerCharacter`))
  (bind _charactermovement (`self.CharacterMovement`))
  (bind _returnvalue (`self.K2_GetActorLocation` _ownercharacter))
  (bind _returnvalue_2 (`self.K2_GetActorLocation` (`/Game/Main/BP_BaseCharacter.LockOnTarget` _ownercharacter)))
  ;[1 1 1] Initialize
  (`parent.Initialize`)
  (for (_array_element _array_index) (`self.Hitboxes`)
    (set `/Game/Misc/BP_Hitbox.HitData` (make `/Game/Main/Structs/Struct_HitData` 0 (0.0 0.0 200.0) 5.0 1 0.001 0.02 1.0) _array_element)
    (`SphereComponent.SetSphereRadius` (`/Game/Misc/BP_Hitbox.Hitbox` _array_element) 75.0 true)
    (`self.K2_SetActorRelativeLocation` _array_element (select `int` _array_index :`0` (100.0 0.0 0.0) :`1` (0.0 0.0 50.0) :`2` (0.0 0.0 -50.0) :!type "Vector Structure") false false)
    (`/Game/Misc/BP_Hitbox.Activate` _array_element true))
  (if (and (`/Game/Main/BP_BaseCharacter.IsLockedOn` _ownercharacter_2) (`KismetSystemLibrary.IsValid` (`/Game/Main/BP_BaseCharacter.LockOnTarget` _ownercharacter_2)))
    (bind _output_get (set `MovementComponent.Velocity` (* (`KismetMathLibrary.GetDirectionUnitVector` _returnvalue _returnvalue_2) (`KismetMathLibrary.VSize` (`MovementComponent.Velocity` _charactermovement))) _charactermovement))
    (set `self.PreviousFrameVelocity` _output_get)
    (`self.K2_SetActorRotation` (`KismetMathLibrary.MakeRotator` (.roll (`self.K2_GetActorRotation`)) (.pitch (`KismetMathLibrary.FindLookAtRotation` _returnvalue _returnvalue_2)) (.yaw (`self.K2_GetActorRotation`))))))

(fn `UserConstructionScript`
  (`parent.UserConstructionScript`))