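; Fire tornado projectile that lingers briefly, pierces targets and hits repeatedly at a rapid rate.
; On Initialize it calls the parent, sets those projectile settings and spawns three large sphere BP_Hitbox actors stacked vertically into a column on the capsule.
; Each hitbox is owned by the projectile, launches straight up, grants no meter and activates immediately.
; An unwired leftover chain for owner attachment, an alternate hitbox and flying movement never runs.
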(event `self.Initialize`
  ;[1 1 1] Initialization
  (`parent.Initialize`)
  (set `self.Duration` 2.0)
  (set `self.MultiHitRate` 0.01)
  (set `self.Piercing` true)
  (for _index (range 3)
    (bind _returnvalue (`|SpawnActorFromClass` "/Game/Misc/BP_Hitbox.BP_Hitbox_C" (`self.GetTransform`) "AlwaysSpawn" "OverrideRootScale" null null))
    (set `/Game/Misc/BP_Hitbox.OwnerCharacter` self _returnvalue)
    (`self.K2_AttachToComponent` _returnvalue (`self.CapsuleComponent`) "None" "KeepWorld" "KeepWorld" "KeepWorld" true)
    (`self.K2_SetActorRelativeLocation` _returnvalue (select `int` _index :`0` (0.0 0.0 0.0) :`1` (0.0 0.0 175.0) :`2` (0.0 0.0 350.0) :!type "Vector Structure") false false)
    (`KismetArrayLibrary.Array_Add` (`self.Hitboxes`) _returnvalue)
    (`SphereComponent.SetSphereRadius` (`/Game/Misc/BP_Hitbox.Hitbox` _returnvalue) 175.0 true)
    (set `/Game/Misc/BP_Hitbox.HitData` (make `/Game/Main/Structs/Struct_HitData` 0 (0.0 0.0 1000.0) 10.0 2 0.05 0.2 0.0) _returnvalue)
    (`/Game/Misc/BP_Hitbox.Activate` _returnvalue true)))

(fn `UserConstructionScript`
  (`parent.UserConstructionScript`))